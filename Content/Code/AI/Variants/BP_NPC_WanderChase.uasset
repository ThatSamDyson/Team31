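; Enemy NPC in a roguelike that randomly tags itself Snap or DontSnap on spawn and drops a coin when destroyed.
; Overlaps damage the player on a cooldown or apply bullet damage to itself, with Ra bullets starting a timer-driven burn.
; On lethal damage it checks the player's relics: Scarab heals the player, and Apep triggers a sphere-trace blast damaging nearby enemies, wider if burning.
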(event OnComponentBeginOverlap()
  (params (OverlappedComponent :type Primitive%20Component%20Object%20Reference) (OtherActor :type Actor%20Object%20Reference) (OtherComp :type Primitive%20Component%20Object%20Reference) (OtherBodyIndex :type Integer) (bFromSweep :type Boolean) (SweepResult :type Hit%20Result%20Structure%20%28by%20ref%29))
  ;[1 1 1] Burn over time damage blueprint
  (bind _output_get (Variables|Default|SetOther%20Actor OtherActor))
  (if (Utilities|DoesObjectImplementInterface _output_get "/Game/Code/Interfaces/BI_Character.BI_Character_C")
    (Utilities|FlowControl|DoOnce false :!label _label
      (:Completed
        (CallFunction|DamagePlayer (Variables|Default|GetDamage))
        (Utilities|FlowControl|Delay 3.0)
        (goto _label Reset)))
    (elif (Utilities|DoesObjectImplementInterface (Variables|Default|GetOther%20Actor) "/Game/Code/Interfaces/BI_Bullet.BI_Bullet_C")
      (Game|Damage|ApplyDamage self 35.0 0 0)
      (if (Utilities|DoesObjectImplementInterface (Variables|Default|GetOther%20Actor) "/Game/Code/Interfaces/BI_Ra.BI_Ra_C")
        (bind _returnvalue (Utilities|Time|SetTimerbyEvent (delegate Custom|BurnDamage) 1.0 true))
        (Variables|Default|SetBurnTimer _returnvalue)
        (Variables|Default|SetOnFire true)))))

(event Custom|BurnDamage
  ;[1 1 1] Burn over time damage blueprint
  (Game|Damage|ApplyDamage self 5.0 0 0)
  (bind _output_get (Variables|Default|SetBurnTime (+ (Variables|Default|GetBurnTime) 1.0)))
  (if (>= _output_get 5.0)
    (Utilities|Time|ClearandInvalidateTimerbyHandle (Variables|Default|GetBurnTimer))
    (Variables|Default|SetOnFire false)))

(event Custom|ApepWarDagger
  (bind _returnvalue (Transformation|GetActorLocation))
  ;[1 1 1] Apeps War Dagger Code
  (if (Variables|Default|GetOnFire)
    (Variables|Default|SetExplosionRadius 4e+02)
    (else
      (Variables|Default|SetExplosionRadius 2e+02)))
  (bind _outhits (Collision|MultiSphereTraceForObjects _returnvalue _returnvalue (Variables|Default|GetExplosionRadius) (Utilities|Array|MakeArray "ObjectTypeQuery3") false 0 "Persistent"))
  (for _array_element _outhits
    (if (Utilities|DoesObjectImplementInterface (.HitActor (Collision|BreakHitResult _array_element)) "/Game/Code/Interfaces/BI_Enemy.BI_Enemy_C")
      (Game|Damage|ApplyDamage (.HitActor (Collision|BreakHitResult _array_element)) 9e+01 0 0)
      (Development|PrintString "Damaged")))
  (Actor|DestroyActor))

(event Custom|Scarab%20Ring
  ;[1 1 1] Scarab Ring. Heal player on death
  (bind _returnvalue (Actor|GetActorOfClass "/Game/Code/Character/CharacterBlueprints/CH_Roguelike.CH_Roguelike_C"))
  (if (> (+ (Variables|/Game/Code/Character/CharacterBlueprints/CH_Roguelike.CH_Roguelike_C|GetplayerHealth _returnvalue) 15.0) 1e+02)
    (bind _returnvalue_2 (Actor|GetActorOfClass "/Game/Code/Character/CharacterBlueprints/CH_Roguelike.CH_Roguelike_C"))
    (CallFunction|DamagePlayer (- 1e+02 (Variables|/Game/Code/Character/CharacterBlueprints/CH_Roguelike.CH_Roguelike_C|GetplayerHealth _returnvalue_2)))
    (else
      (CallFunction|DamagePlayer -15.0))))

(event Game|Damage|EventAnyDamage
  (params (Damage :type Float%20%28single-precision%29) (DamageType :type Damage%20Type%20Object%20Reference) (InstigatedBy :type Controller%20Object%20Reference) (DamageCauser :type Actor%20Object%20Reference))
  (bind _output_get (Variables|Default|SetHealth (- (Variables|Default|GetHealth) Damage)))
  (if (<= _output_get 0.0)
    (bind _returnvalue (Actor|GetActorOfClass "/Game/Code/Character/CharacterBlueprints/CH_Roguelike.CH_Roguelike_C"))
    (if (Variables|/Game/Code/Character/CharacterBlueprints/CH_Roguelike.CH_Roguelike_C|GetHasScarab _returnvalue)
      (CallFunction|ScarabRing))
    (if (Variables|/Game/Code/Character/CharacterBlueprints/CH_Roguelike.CH_Roguelike_C|GetHasApep _returnvalue)
      (CallFunction|ApepWarDagger)
      (else
        (Actor|DestroyActor)))))

(event EventBeginPlay
  (if (>= (Math|Random|RandomIntegerinRange 0 1) 1)
    (Variables|Default|SetTags (Variables|Default|GetSnap))
    (else
      (Variables|Default|SetTags (Variables|Default|GetDon't%20Snap)))))

(event EventDestroyed
  ;[1 1 1] Item drop
  (Game|SpawnActorfromClass "/Game/Code/Objects/BP_Coin.BP_Coin_C" (Transformation|GetActorTransform) "Undefined" "MultiplyWithRoot" 0 0))

(fn ConstructionScript)

(fn TakeDamage
  (params (Damage :type Float%20%28double-precision%29))
  (bind _returnvalue (Transformation|GetActorLocation))
  (bind _output_get (Variables|Default|SetHealth (- (Variables|Default|GetHealth) Damage)))
  (if (<= _output_get 0.0)
    (bind _returnvalue_2 (Actor|GetActorOfClass "/Game/Code/Character/CharacterBlueprints/CH_Roguelike.CH_Roguelike_C"))
    (if (Variables|/Game/Code/Character/CharacterBlueprints/CH_Roguelike.CH_Roguelike_C|GetHasApep _returnvalue_2)
      (if (Variables|Default|GetOnFire)
        (Variables|Default|SetExplosionRadius 4e+02)
        (else
          (Variables|Default|SetExplosionRadius 2e+02)))
      (bind _outhits (Collision|MultiSphereTraceForObjects _returnvalue _returnvalue (Variables|Default|GetExplosionRadius) (Utilities|Array|MakeArray "ObjectTypeQuery3") false 0 "Persistent"))
      (for _array_element _outhits
        (if (Utilities|DoesObjectImplementInterface (.HitActor (Collision|BreakHitResult _array_element)) "/Game/Code/Interfaces/BI_Enemy.BI_Enemy_C")
          _)))
    (Actor|DestroyActor)))

(fn DamagePlayer
  (params (Damage :type Float%20%28double-precision%29))
  (bind _returnvalue (Actor|GetActorOfClass "/Game/Code/Character/CharacterBlueprints/CH_Roguelike.CH_Roguelike_C"))
  (Default|TakeDamage _returnvalue Damage))