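; Two-phase boss NPC that hurts the player on contact and takes damage from bullets, randomly tagged Snap or DontSnap at spawn.
; Component overlaps route by interface: characters trigger damage to the CH_Roguelike actor on a three-second cooldown, bullets reduce boss health.
; Reaching the phase-two threshold refills health and spawns BP_NPC_WanderChase minions at an offset.
; Depleting health in phase two destroys the boss.
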(event OnComponentBeginOverlap()
  (params (OverlappedComponent :type Primitive%20Component%20Object%20Reference) (OtherActor :type Actor%20Object%20Reference) (OtherComp :type Primitive%20Component%20Object%20Reference) (OtherBodyIndex :type Integer) (bFromSweep :type Boolean) (SweepResult :type Hit%20Result%20Structure%20%28by%20ref%29))
  (if (Utilities|DoesObjectImplementInterface OtherActor "/Game/Code/Interfaces/BI_Character.BI_Character_C")
    (Utilities|FlowControl|DoOnce false :!label _label
      (:Completed
        (CallFunction|DamagePlayer)
        (Utilities|FlowControl|Delay 3.0)
        (goto _label Reset)))
    (elif (Utilities|DoesObjectImplementInterface OtherActor "/Game/Code/Interfaces/BI_Bullet.BI_Bullet_C")
      (Utilities|FlowControl|DoOnce false :!label _label_2
        (:Completed
          (CallFunction|TakeDamage)
          (goto _label_2 Reset))))))

(event Collision|EventActorBeginOverlap
  (params (OtherActor :type Actor%20Object%20Reference)))

(event EventTick
  (params (DeltaSeconds :type Float%20%28single-precision%29)))

(event EventBeginPlay
  (if (>= (Math|Random|RandomIntegerinRange 0 1) 1)
    (Variables|Default|SetTags (Variables|Default|GetSnap))
    (else
      (Variables|Default|SetTags (Variables|Default|GetDon't%20Snap)))))

(fn ConstructionScript)

(fn TakeDamage
  (if (Variables|Default|GetisPhase2)
    (bind _output_get (Variables|Default|SetHealth (- (Variables|Default|GetHealth) (Variables|Default|GetBulletDamage))))
    (Development|PrintString (Utilities|String|ToString(Float) (Variables|Default|GetHealth)))
    (if (and (<= _output_get 0.0) (Variables|Default|GetisPhase2))
      (Actor|DestroyActor))
    (else
      (bind _output_get_2 (Variables|Default|SetHealth (- (Variables|Default|GetHealth) (Variables|Default|GetBulletDamage))))
      (Development|PrintString (Utilities|String|ToString(Float) (Variables|Default|GetHealth)))
      (if (and (<= _output_get_2 (Variables|Default|GetHealthPhase2)) (not (Variables|Default|GetisPhase2)))
        (Variables|Default|SetisPhase2 true)
        (Variables|Default|SetHealth (Variables|Default|GetMaxHealth))
        (Utilities|FlowControl|ForLoopwithBreak 0 (Variables|Default|GetEnemyAmount)
          (:LoopBody
            (Game|SpawnActorfromClass "/Game/Code/AI/Variants/BP_NPC_WanderChase.BP_NPC_WanderChase_C" (Math|Transform|MakeTransform (+ (.location (Transformation|GetActorTransform)) (Variables|Default|GetSpawn%20Offset)) "0, 0, 0" "1.000000,1.000000,1.000000") "AdjustIfPossibleButAlwaysSpawn" "MultiplyWithRoot" 0 0))
          (:Completed
            (Development|PrintString "Hello")))))))

(fn DamagePlayer
  (bind _returnvalue (Actor|GetActorOfClass "/Game/Code/Character/CharacterBlueprints/CH_Roguelike.CH_Roguelike_C"))
  (Default|TakeDamage _returnvalue (Variables|Default|GetDamage)))