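; Base enemy NPC that deals contact damage to the CH_Roguelike player and is destroyed when bullets deplete its health.
; Collide overlap and hit events use BI_Character and BI_Bullet interface checks to choose between damaging the player and losing one health.
; Overlap damage to the player has a three-second DoOnce cooldown, while hit events are ungated.
; The player is found with GetActorOfClass rather than taken from the colliding actor.
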(event OnComponentHit(Collide)
  (params (HitComponent :type Primitive%20Component%20Object%20Reference) (OtherActor :type Actor%20Object%20Reference) (OtherComp :type Primitive%20Component%20Object%20Reference) (NormalImpulse :type Vector :default "0, 0, 0") (Hit :type Hit%20Result%20Structure%20%28by%20ref%29))
  (if (Utilities|DoesObjectImplementInterface OtherActor "/Game/Code/Interfaces/BI_Character.BI_Character_C")
    (CallFunction|DamagePlayer)
    (Utilities|FlowControl|Delay 0.25)
    (elif (Utilities|DoesObjectImplementInterface OtherActor "/Game/Code/Interfaces/BI_Bullet.BI_Bullet_C")
      (CallFunction|TakeDamage))))

(event OnComponentBeginOverlap(Collide)
  (params (OverlappedComponent :type Primitive%20Component%20Object%20Reference) (OtherActor :type Actor%20Object%20Reference) (OtherComp :type Primitive%20Component%20Object%20Reference) (OtherBodyIndex :type Integer) (bFromSweep :type Boolean) (SweepResult :type Hit%20Result%20Structure%20%28by%20ref%29))
  (if (Utilities|DoesObjectImplementInterface OtherActor "/Game/Code/Interfaces/BI_Character.BI_Character_C")
    (Utilities|FlowControl|DoOnce false :!label _label
      (:Completed
        (CallFunction|DamagePlayer)
        (Utilities|FlowControl|Delay 3.0)
        (goto _label Reset)))
    (elif (Utilities|DoesObjectImplementInterface OtherActor "/Game/Code/Interfaces/BI_Bullet.BI_Bullet_C")
      (Utilities|FlowControl|DoOnce false :!label _label_2
        (:Completed
          (CallFunction|TakeDamage)
          (goto _label_2 Reset))))))

(event Custom|Take%20Damage
  (bind _output_get (Variables|Default|SetHealth (- (Variables|Default|GetHealth) 1.0)))
  (if (<= _output_get 0.0)
    (Actor|DestroyActor)))

(event Custom|Damage%20Player
  (bind _returnvalue (Actor|GetActorOfClass "/Game/Code/Character/CharacterBlueprints/CH_Roguelike.CH_Roguelike_C"))
  (Default|TakeDamage _returnvalue (Variables|Default|GetDamage)))

(event EventBeginPlay)

(event Collision|EventActorBeginOverlap
  (params (OtherActor :type Actor%20Object%20Reference)))

(event EventTick
  (params (DeltaSeconds :type Float%20%28single-precision%29)))

(fn ConstructionScript)