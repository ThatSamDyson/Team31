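; BP_Room is a procedurally generated room actor that builds its floor, walls and doors on BeginPlay.
; Generation lays a grid of floor instances, then walks the four edges, leaving one opening at the first bottom-edge slot unless OriginRoom is set.
; At every other edge slot, SpawnDoor rolls the DoorSeed stream, weighted by desired and existing door counts.
; It spawns a BP_Door into DoorArray, or otherwise adds a wall instance.
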(event EventBeginPlay
  (CallFunction|Generation))

(fn ConstructionScript)

(fn Generation
  ;[1 1 1] Floor Generation
  ;;[1 1 1] Row Generation
  (for _index (range 0 (- (Variables|Default|GetFloorTilesY) 1))
    ;;[1 1 1] Column Generation
    (for _index_2 (range 0 (- (Variables|Default|GetFloorTilesX) 1))
      (Components|InstancedStaticMesh|AddInstance (Variables|Default|GetFloor) (Math|Transform|MakeTransform (Math|Vector|MakeVector (* _index_2 (Variables|Default|GetFloorSizeX)) (* (Variables|Default|GetFloorSizeY) _index) 0.0) "0, 0, 0" "1.000000,1.000000,1.000000") false)))
  ;[1 1 1] Wall Generation
  (for _index_3 (range 0 (- (Variables|Default|GetFloorTilesY) 1))
    ;[1 1 1] Starting Room Check
    (if (or (!= _index_3 0) (Variables|Default|GetOriginRoom))
      ;;[1 1 1] Bottom Wall Generation
      (CallFunction|SpawnDoor (== (Math|Integer|%(Integer) _index_3 2) 1) (Math|Vector|MakeVector 0.0 (* _index_3 (Variables|Default|GetFloorSizeY)) 0.0) "0.000000,90.000000,0.000000"))
    ;;[1 1 1] Top Wall Generation
    (CallFunction|SpawnDoor (== (Math|Integer|%(Integer) _index_3 2) 1) (Math|Vector|MakeVector (* (Variables|Default|GetFloorTilesX) (Variables|Default|GetFloorSizeX)) (* (Variables|Default|GetFloorSizeY) (+ _index_3 1)) 0.0) "0.000000,-90.000000,0.000000"))
  (for _index_4 (range 0 (- (Variables|Default|GetFloorTilesX) 1))
    ;;[1 1 1] Right Wall Generation
    (CallFunction|SpawnDoor (== (Math|Integer|%(Integer) _index_4 2) 1) (Math|Vector|MakeVector (* _index_4 (Variables|Default|GetFloorSizeX)) (* (Variables|Default|GetFloorSizeY) (Variables|Default|GetFloorTilesY)) 0.0) "0, 0, 0")
    ;;[1 1 1] Left Wall Generation
    (CallFunction|SpawnDoor (== (Math|Integer|%(Integer) _index_4 2) 1) (Math|Vector|MakeVector (* (Variables|Default|GetFloorSizeX) (+ _index_4 1)) 0.0 0.0) "0.000000,180.000000,0.000000")))

(fn SpawnDoor
  (params (CanSpawnDoor :type Boolean) (Location :type Vector) (Rotation :type Rotator))
  (bind _returnvalue (Transformation|GetActorTransform))
  (bind _desireddooramount (Variables|Default|GetDesiredDoorAmount))
  ;[1 1 1] Is Door Check
  (if (and CanSpawnDoor (Class|KismetMathLibrary|RandomBoolwithWeightfromStream (Variables|Default|GetDoorSeed) (Math|Conversions|ToFloat(Integer) (/ _desireddooramount (- _desireddooramount (Utilities|Array|Length (Variables|Default|GetDoorArray)))))))
    ;[1 1 1] Spawn and transform spawned door to world space then add to an array of all spawned doors
    (bind _returnvalue_2 (Game|SpawnActorfromClass "/Game/Code/PCGLevel/Blueprints/BP_Door.BP_Door_C" (Math|Transform|MakeTransform (Math|Transform|TransformLocation _returnvalue Location) (Math|Transform|TransformRotation _returnvalue Rotation) "1.000000,1.000000,1.000000") "Undefined" "MultiplyWithRoot" 0 0))
    (Utilities|Array|Add (Variables|Default|GetDoorArray) _returnvalue_2)
    (else
      ;[1 1 1] Add wall instead of door
      (Components|InstancedStaticMesh|AddInstance (Variables|Default|GetWall) (Math|Transform|MakeTransform Location Rotation "1.000000,1.000000,1.000000") false))))