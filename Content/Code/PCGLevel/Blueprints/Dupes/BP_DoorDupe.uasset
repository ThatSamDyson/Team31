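; Procedural-level door that swings open and closed on Activate, spawning a BP_RoomDupe behind it on first opening if still allowed.
; A line trace hitting another door or wall collision produces a connecting hallway, disabling that door's generation or removing that wall piece.
; Otherwise, side traces measure free space to size and offset a new room.
; A seeded stream drives dimensions, door counts and child seeds; OldGenerateNewRoom is legacy.
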(event Custom|GenerateNewRoom
  (params (RoomTileY :type Integer) (RoomTileX :type Integer) (MaxDoors :type Integer) (Shift :type Integer) (Hallway :type Boolean))
  (Game|SpawnActorfromClass "/Game/Code/PCGLevel/Blueprints/Dupes/BP_RoomDupe.BP_RoomDupe_C" (Math|Transform|MakeTransform (+ (Transformation|GetActorLocation) (* (Transformation|GetActorForwardVector) 4e+02) (* (Transformation|GetActorRightVector) 4e+02)) (Math|Rotator|CombineRotators (Transformation|GetActorRotation) "0.000000,90.000000,0.000000") "1.000000,1.000000,1.000000") "Undefined" "MultiplyWithRoot" 0 RoomTileY RoomTileX MaxDoors Shift Hallway (Class|KismetMathLibrary|RandomIntegerfromStream (Variables|Default|GetDoorStream) 100000) 0))

(event Custom|AddAdditional
  (bind _returnvalue (Transformation|GetActorTransform))
  (bind _returnvalue_2 (Transformation|GetActorForwardVector))
  (bind _roomsizelimit (Variables|Default|GetRoomSizeLimit))
  (bind _tilesize (Variables|Default|GetTileSize))
  (bind _returnvalue_3 (Math|Transform|TransformLocation _returnvalue "200.000000,10.000000,200.000000"))
  (bind _returnvalue_4 (- _roomsizelimit 1))
  (bind _returnvalue_5 (* _returnvalue_4 _tilesize))
  (bind _returnvalue_6 (* _returnvalue_2 _returnvalue_5))
  (bind (_outhit _returnvalue_7) (Collision|LineTraceByChannel _returnvalue_3 (+ _returnvalue_3 (* (Transformation|GetActorRightVector) (* (Variables|Default|GetRoomSizeLimit) (Variables|Default|GetTileSize)))) "TraceTypeQuery1" false 0 "Persistent"))
  (if _returnvalue_7
    (switch string (Utilities|GetClassDisplayName (Utilities|GetClass (.HitActor (Collision|BreakHitResult _outhit))))
      (:BP_DoorDupe_C
        (bind _asbp_door_dupe (Utilities|Casting|CastToBP_DoorDupe (.HitActor (Collision|BreakHitResult _outhit))))
        (Variables|BP_DoorDupe_C|SetCanRoom _asbp_door_dupe false))
      (:BP_WallCollisionDupe_C
        (bind _asbp_wall_collision_dupe (Utilities|Casting|CastToBP_WallCollisionDupe (.HitActor (Collision|BreakHitResult _outhit))))
        (Default|RemoveIndex _asbp_wall_collision_dupe)))
    (CallFunction|GenerateNewRoom 1 (- (Math|Float|Round (/ (.Distance (Collision|BreakHitResult _outhit)) (Variables|Default|GetTileSize))) 1) (Math|Random|RandomIntegerinRangefromStream (Variables|Default|GetDoorStream) 0 2) 0 true)
    (else
      (for _index (range 1 (- (Variables|Default|GetRoomSizeLimit) 1))
        (Utilities|FlowControl|Sequence
          (:then_0
            (bind (_outhit_2 _returnvalue_8) (Collision|LineTraceByChannel (Math|Transform|TransformLocation (Transformation|GetActorTransform) (+ "390.000000,200.000000,300.000000" (Math|Vector|MakeVector 0.0 (* _index 4e+02) 0.0))) (+ (Math|Transform|TransformLocation (Transformation|GetActorTransform) (+ "390.000000,200.000000,300.000000" (Math|Vector|MakeVector 0.0 (* _index 4e+02) 0.0))) _returnvalue_6) "TraceTypeQuery1" false 0 "Persistent"))
            (if _returnvalue_8
              (Variables|Default|SetLeftLimit (Math|Integer|Min(Integer) (Math|Float|Round (/ (.Distance (Collision|BreakHitResult _outhit_2)) (Variables|Default|GetTileSize))) (Variables|Default|GetLeftLimit)))))
          (:then_1
            (bind (_outhit_3 _returnvalue_9) (Collision|LineTraceByChannel (Math|Transform|TransformLocation (Transformation|GetActorTransform) (+ "10.000000,200.000000,300.000000" (Math|Vector|MakeVector 0.0 (* _index 4e+02) 0.0))) (+ (Math|Transform|TransformLocation (Transformation|GetActorTransform) (+ "10.000000,200.000000,300.000000" (Math|Vector|MakeVector 0.0 (* _index 4e+02) 0.0))) (* _returnvalue_6 -1.0)) "TraceTypeQuery1" false 0 "Persistent"))
            (if _returnvalue_9
              (Variables|Default|SetRightLimit (Math|Integer|Min(Integer) (Math|Float|Round (/ (.Distance (Collision|BreakHitResult _outhit_3)) (Variables|Default|GetTileSize))) (Variables|Default|GetRightLimit)))))))
      (Variables|Default|SetSpace (Math|Random|RandomIntegerinRangefromStream (Variables|Default|GetDoorStream) 0 (Math|Integer|Min(Integer) (+ (Variables|Default|GetRightLimit) (Variables|Default|GetLeftLimit)) (Variables|Default|GetRoomSizeLimit))))
      (Variables|Default|SetShift (Math|Random|RandomIntegerinRangefromStream (Variables|Default|GetDoorStream) (Math|Integer|Clamp(Integer) (- (Variables|Default|GetSpace) (Variables|Default|GetRightLimit)) 0 (Variables|Default|GetSpace)) (Math|Integer|Min(Integer) (Variables|Default|GetSpace) (Variables|Default|GetLeftLimit))))
      (CallFunction|GenerateNewRoom (+ (Variables|Default|GetSpace) 1) (Math|Random|RandomIntegerinRangefromStream (Variables|Default|GetDoorStream) 3 (Variables|Default|GetRoomSizeLimit)) (Math|Random|RandomIntegerinRangefromStream (Variables|Default|GetDoorStream) 3 6) (Variables|Default|GetShift) false))))

(event Custom|OldGenerateNewRoom
  ;[1 1 1] Old
  (Variables|Default|SetRandomRoomX (Math|Random|RandomIntegerinRange 3 8))
  (Variables|Default|SetRandomRoomY (Math|Random|RandomIntegerinRange 3 8))
  (Variables|Default|SetRandomDoorValue (Math|Random|RandomIntegerinRange 4 6))
  (Game|SpawnActorfromClass "/Game/Code/PCGLevel/Blueprints/Dupes/BP_RoomDupe.BP_RoomDupe_C" (Math|Transform|MakeTransform (+ (Transformation|GetActorLocation) (* (Transformation|GetActorForwardVector) 4e+02)) (Math|Rotator|CombineRotators (Transformation|GetActorRotation) "0.000000,90.000000,0.000000") "1.000000,1.000000,1.000000") "Undefined" "MultiplyWithRoot" 0 (Variables|Default|GetRandomRoomY) (Variables|Default|GetRandomRoomX) (Variables|Default|GetRandomDoorValue) 0 false 0 0))

(event EventBeginPlay
  (Variables|Default|SetDoorStream (Math|Random|MakeRandomStream (Variables|Default|GetSeed))))

(event EventActivate
  (if (Variables|Default|GetClosed)
    (Variables|Default|SetClosed false)
    (Utilities|FlowControl|Sequence
      (:then_0
        (if (Variables|Default|GetCanRoom)
          (Variables|Default|SetCanRoom false)
          (bind _output_get (Variables|Default|SetRoomSizeLimit (Math|Random|RandomIntegerinRangefromStream (Variables|Default|GetDoorStream) 3 10)))
          (bind _output_get_2 (Variables|Default|SetLeftLimit _output_get))
          (Variables|Default|SetRightLimit _output_get_2)
          (CallFunction|AddAdditional)))
      (:then_1
        (bind _doortrack (Timeline|DoorSwingTimeline Play)
          (:Update
            (Transformation|SetRelativeRotation (Variables|Default|GetHinge) (Math|Rotator|MakeRotator 0.0 0.0 _doortrack) false false)))))
    (else
      (Variables|Default|SetClosed true)
      (Timeline|DoorSwingTimeline Reverse))))

(fn ConstructionScript)