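; Procedural roguelike dungeon room that builds itself on BeginPlay from a tile grid.
; Floor tiles randomly receive pit or other traps, enemies and props, with trap and prop classes sampled from tagged world actors; shop rooms spawn a shop instead.
; Edges become stream-randomized doors or instanced walls with collision actors, which RemoveWall uses index swapping to maintain.
; Line traces detect existing geometry to prevent overlaps and disable room spawning on hit doors.
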(event Custom|RemoveWall
  (params (Index :type Integer))
  (bind _wallcollision (Variables|Default|GetWallCollision))
  (bind _returnvalue (Utilities|Array|LastIndex _wallcollision))
  (bind _output (Utilities|Array|Get(acopy) _wallcollision _returnvalue))
  ;[1 1 1] Removes a wall after a hallway is determined to be needed
  (Class|InstancedStaticMeshComponent|RemoveInstance (Variables|Default|GetHeirarchWall) Index)
  (Utilities|Array|SetArrayElem _wallcollision Index _output true)
  (Default|Update _output Index)
  (Utilities|Array|RemoveIndex (Variables|Default|GetWallCollision) _returnvalue))

(event EventBeginPlay
  ;[1 1 1] Generates a new seed based off of a start value
  (bind _asgm_roguelike (Utilities|Casting|CastToGM_Roguelike (Game|GetGameMode)))
  (Variables|Default|SetGameMode _asgm_roguelike)
  (Variables|Default|SetDoorSeed (Math|Random|MakeRandomStream (+ (Variables|Default|GetStartSeed) (Math|Random|RandomIntegerinRange 1 100000))))
  (Utilities|FlowControl|Sequence
    (:then_0
      (Utilities|FlowControl|DoOnce false
        (:Completed
          (Utilities|FlowControl|Sequence
            (:then_0
              ;[1 1 1] Gets all the world traps on room spawn that are tagged
              (bind _outactors (Actor|GetAllActorswithTag "Trap"))
              (for _array_element _outactors
                (Utilities|Array|AddUnique (Variables|Default|GetTrapArray) _array_element)))
            (:then_1
              (bind _outactors_2 (Actor|GetAllActorswithTag "Prop"))
              (for _array_element_2 _outactors_2
                (Utilities|Array|AddUnique (Variables|Default|GetPropArray) _array_element_2)))))))
    (:then_1
      (CallFunction|Generation))))

(fn ConstructionScript)

(fn Generation
  ;[0.9844 1 0.9688] Floor Generation
  ;;[1 1 1] Row Generation
  (for _index (range 0 (- (Variables|Default|GetFloorTilesY) 1))
    ;;[1 1 1] Column Generation
    (for _index_2 (range 0 (- (Variables|Default|GetFloorTilesX) 1))
      (bind (_pittrap _trapped) (CallFunction|SpawnTrap (Math|Vector|MakeVector (* _index_2 (Variables|Default|GetFloorSizeX)) (* (Variables|Default|GetFloorSizeY) (- _index (Variables|Default|GetEnterShift))) 0.0)))
      (Variables|Default|SetTrapped _trapped)
      (if (not _pittrap)
        (Components|InstancedStaticMesh|AddInstance (Variables|Default|GetFloor) (Math|Transform|MakeTransform (Math|Vector|MakeVector (* _index_2 (Variables|Default|GetFloorSizeX)) (* (Variables|Default|GetFloorSizeY) (- _index (Variables|Default|GetEnterShift))) 0.0) "0, 0, 0" "1.000000,1.000000,1.000000") false)
        (Rendering|Material|SetMaterialbyName (Variables|Default|GetFloor) "Floor" "/Game/BrickMaterial/Brick_Inst.Brick_Inst")
        (CallFunction|SpawnAi (+ "0.000000,0.000000,44.000000" (Math|Vector|MakeVector (* _index_2 (Variables|Default|GetFloorSizeX)) (* (Variables|Default|GetFloorSizeY) (- _index (Variables|Default|GetEnterShift))) 0.0)))
        (CallFunction|SpawnProps (Math|Vector|MakeVector (* _index_2 (Variables|Default|GetFloorSizeX)) (* (Variables|Default|GetFloorSizeY) (- _index (Variables|Default|GetEnterShift))) 0.0))
        (if (not (Variables|/Game/Code/Gamemodes/GM_Roguelike.GM_Roguelike_C|GetshopSpawned (Variables|Default|GetGameMode)))
          (if (not (Variables|Default|GetOriginRoom))
            (if (Variables|Default|GetisShop)
              (CallFunction|SpawnShop (Math|Vector|MakeVector (* _index_2 (Variables|Default|GetFloorSizeX)) (* (Variables|Default|GetFloorSizeY) (- _index (Variables|Default|GetEnterShift))) 0.0))))))))
  ;[1 1 1] Checks if there is a hallway or not before creating new walls
  (if (not (Variables|Default|GetHallway))
    ;[1 1 1] Wall Generation
    (for _index_3 (range 0 (- (Variables|Default|GetFloorTilesY) 1))
      ;[1 1 1] Starting Room Check
      (if (or (!= _index_3 (Variables|Default|GetEnterShift)) (Variables|Default|GetOriginRoom))
        ;;[0 0.502 1] Bottom Wall Generation
        (CallFunction|SpawnDoor (== (Math|Integer|%(Integer) _index_3 (Variables|Default|GetDoorEvery)) (Variables|Default|GetDoorRemainder)) (- (Math|Vector|MakeVector 0.0 (* _index_3 (Variables|Default|GetFloorSizeY)) 0.0) (Math|Vector|MakeVector 0.0 (* (Variables|Default|GetEnterShift) (Variables|Default|GetFloorSizeY)) 0.0)) "0.000000,90.000000,0.000000"))
      ;;[0 0.502 1] Top Wall Generation
      (CallFunction|SpawnDoor (== (Math|Integer|%(Integer) _index_3 (Variables|Default|GetDoorEvery)) (Variables|Default|GetDoorRemainder)) (- (Math|Vector|MakeVector (* (Variables|Default|GetFloorTilesX) (Variables|Default|GetFloorSizeX)) (* (Variables|Default|GetFloorSizeY) (+ _index_3 1)) 0.0) (Math|Vector|MakeVector 0.0 (* (Variables|Default|GetEnterShift) (Variables|Default|GetFloorSizeY)) 0.0)) "0.000000,-90.000000,0.000000")))
  (for _index_4 (range 0 (- (Variables|Default|GetFloorTilesX) 1))
    ;;[0 0.502 1] Right Wall Generation
    (CallFunction|SpawnDoor (== (Math|Integer|%(Integer) _index_4 (Variables|Default|GetDoorEvery)) (Variables|Default|GetDoorRemainder)) (- (Math|Vector|MakeVector (* _index_4 (Variables|Default|GetFloorSizeX)) (* (Variables|Default|GetFloorSizeY) (Variables|Default|GetFloorTilesY)) 0.0) (Math|Vector|MakeVector 0.0 (* (Variables|Default|GetEnterShift) (Variables|Default|GetFloorSizeY)) 0.0)) "0, 0, 0")
    ;;[0 0.502 1] Left Wall Generation
    (CallFunction|SpawnDoor (== (Math|Integer|%(Integer) _index_4 (Variables|Default|GetDoorEvery)) (Variables|Default|GetDoorRemainder)) (- (Math|Vector|MakeVector (* (Variables|Default|GetFloorSizeX) (+ _index_4 1)) 0.0 0.0) (Math|Vector|MakeVector 0.0 (* (Variables|Default|GetEnterShift) (Variables|Default|GetFloorSizeY)) 0.0)) "0.000000,180.000000,0.000000"))
  ;[1 1 1] Adds one gap spacing for room entrance
  (if (not (Variables|Default|GetOriginRoom))
    (CallFunction|SpacingHallway)))

(fn SpawnDoor
  (params (CanSpawnDoor :type Boolean) (Location :type Vector) (Rotation :type Rotator))
  (bind _returnvalue (Transformation|GetActorTransform))
  (bind _desireddooramount (Variables|Default|GetDesiredDoorAmount))
  (bind _returnvalue_2 (Math|Transform|TransformLocation _returnvalue Location))
  (bind _returnvalue_3 (Math|Transform|TransformRotation _returnvalue Rotation))
  ;[1 1 1] Check for walls overlapping doors
  (Utilities|OverlappingDoorandWall Location Rotation
    (:False
      ;[1 1 1] Is Door Check
      (if (and CanSpawnDoor (Class|KismetMathLibrary|RandomBoolwithWeightfromStream (Variables|Default|GetDoorSeed) (/ _desireddooramount (- _desireddooramount (Utilities|Array|Length (Variables|Default|GetDoorArray))))))
        ;[1 1 1] Spawn and transform spawned door to world space then add to an array of all spawned doors
        (bind _returnvalue_4 (Game|SpawnActorfromClass "/Game/Code/PCGLevel/Blueprints/Dupes/BP_DoorDupe.BP_DoorDupe_C" (Math|Transform|MakeTransform _returnvalue_2 _returnvalue_3 "1.000000,1.000000,1.000000") "Undefined" "MultiplyWithRoot" 0 (Class|KismetMathLibrary|RandomIntegerfromStream (Variables|Default|GetDoorSeed) 10000) 0))
        (Rendering|Material|SetMaterialbyName (Variables|/Game/Code/PCGLevel/Blueprints/Dupes/BP_DoorDupe.BP_DoorDupe_C|GetFrame _returnvalue_4) "Wall" "/Game/Art/Materials/SandStoneWall/Wall1_Inst.Wall1_Inst")
        (Rendering|Material|SetMaterialbyName (Variables|/Game/Code/PCGLevel/Blueprints/Dupes/BP_DoorDupe.BP_DoorDupe_C|GetFrame _returnvalue_4) "Sand" "/Game/Art/Materials/sand/MM_Sand_Inst.MM_Sand_Inst")
        (Utilities|Array|Add (Variables|Default|GetDoorArray) _returnvalue_4)
        (else
          ;[1 1 1] Add wall instead of door
          (bind _returnvalue_5 (Components|InstancedStaticMesh|AddInstance (Variables|Default|GetHeirarchWall) (Math|Transform|MakeTransform Location Rotation "1.000000,1.000000,1.000000") false))
          (Components|InstancedStaticMesh|AddInstance (Variables|Default|GetCornerPiece) (Math|Transform|MakeTransform Location (Math|Rotator|CombineRotators Rotation "0.000000,90.000000,0.000000") "1.000000,1.000000,1.000000") false)
          (Rendering|Material|SetMaterial (Variables|Default|GetCornerPiece) 0 "/Game/Art/Materials/Corner/MMcorner_Inst.MMcorner_Inst")
          (Rendering|Material|SetMaterialbyName (Variables|Default|GetHeirarchWall) "Wall" "/Game/Art/Materials/SandStoneWall/Wall1_Inst.Wall1_Inst")
          (Rendering|Material|SetMaterialbyName (Variables|Default|GetHeirarchWall) "Sand" "/Game/Art/Materials/sand/MM_Sand_Inst.MM_Sand_Inst")
          (Rendering|Material|SetMaterialbyName (Variables|Default|GetHeirarchWall) "Not_Seen" "/Game/Art/Materials/sand/MM_Sand_Inst.MM_Sand_Inst")
          (bind _returnvalue_6 (Game|SpawnActorfromClass "/Game/Code/PCGLevel/Blueprints/Dupes/BP_WallCollisionDupe.BP_WallCollisionDupe_C" (Math|Transform|MakeTransform _returnvalue_2 _returnvalue_3 "1.000000,1.000000,1.000000") "Undefined" "MultiplyWithRoot" 0 _returnvalue_5 self 0))
          (Utilities|Array|AddUnique (Variables|Default|GetWallCollision) _returnvalue_6))))))

(fn SpacingHallway
  (bind _returnvalue (Transformation|GetActorTransform))
  (bind _returnvalue_2 (Transformation|GetActorTransform))
  (Utilities|FlowControl|Sequence
    (:then_0
      ;[1 1 1] Add right wall wall to entry zone
      (Utilities|OverlappingDoorandWall "-200.000000,200.000000,0.000000"
        (:False
          (bind _returnvalue_3 (Components|InstancedStaticMesh|AddInstance (Variables|Default|GetHeirarchWall) (Math|Transform|MakeTransform "-200.000000,200.000000,0.000000" "0, 0, 0" "1.000000,1.000000,1.000000") false))
          (Rendering|Material|SetMaterialbyName (Variables|Default|GetHeirarchWall) "Wall" "/Game/Art/Materials/SandStoneWall/Wall1_Inst.Wall1_Inst")
          (Rendering|Material|SetMaterialbyName (Variables|Default|GetHeirarchWall) "Sand" "/Game/Art/Materials/sand/MM_Sand_Inst.MM_Sand_Inst")
          (Rendering|Material|SetMaterialbyName (Variables|Default|GetHeirarchWall) "Not_Seen" "/Game/Art/Materials/sand/MM_Sand_Inst.MM_Sand_Inst")
          (bind _returnvalue_4 (Game|SpawnActorfromClass "/Game/Code/PCGLevel/Blueprints/Dupes/BP_WallCollisionDupe.BP_WallCollisionDupe_C" (Math|Transform|MakeTransform (Math|Transform|TransformLocation _returnvalue_2 "-200.000000,200.000000,0.000000") (Math|Transform|TransformRotation _returnvalue_2 "0, 0, 0") "1.000000,1.000000,1.000000") "Undefined" "MultiplyWithRoot" 0 _returnvalue_3 self 0))
          (Utilities|Array|AddUnique (Variables|Default|GetWallCollision) _returnvalue_4))))
    (:then_1
      ;[1 1 1] Add left wall for entry zone
      (Utilities|OverlappingDoorandWall :Rotation "0.000000,180.000000,0.000000"
        (:False
          (bind _returnvalue_5 (Components|InstancedStaticMesh|AddInstance (Variables|Default|GetHeirarchWall) (Math|Transform|MakeTransform "0, 0, 0" "0.000000,180.000000,0.000000" "1.000000,1.000000,1.000000") false))
          (Rendering|Material|SetMaterialbyName (Variables|Default|GetHeirarchWall) "Wall" "/Game/Art/Materials/SandStoneWall/Wall1_Inst.Wall1_Inst")
          (Rendering|Material|SetMaterialbyName (Variables|Default|GetHeirarchWall) "Sand" "/Game/Art/Materials/sand/MM_Sand_Inst.MM_Sand_Inst")
          (Rendering|Material|SetMaterialbyName (Variables|Default|GetHeirarchWall) "Not_Seen" "/Game/Art/Materials/sand/MM_Sand_Inst.MM_Sand_Inst")
          (bind _returnvalue_6 (Game|SpawnActorfromClass "/Game/Code/PCGLevel/Blueprints/Dupes/BP_WallCollisionDupe.BP_WallCollisionDupe_C" (Math|Transform|MakeTransform (Math|Transform|TransformLocation _returnvalue "0, 0, 0") (Math|Transform|TransformRotation _returnvalue "0.000000,180.000000,0.000000") "1.000000,1.000000,1.000000") "Undefined" "MultiplyWithRoot" 0 _returnvalue_5 self 0))
          (Utilities|Array|AddUnique (Variables|Default|GetWallCollision) _returnvalue_6))))
    (:then_2
      ;[1 1 1] Add new floor for spacing section
      (Components|InstancedStaticMesh|AddInstance (Variables|Default|GetFloor) (Math|Transform|MakeTransform "-200.000000,0.000000,0.000000" "0, 0, 0" "1.000000,1.000000,1.000000") false)
      (Rendering|Material|SetMaterialbyName (Variables|Default|GetFloor) "Floor" "/Game/BrickMaterial/Brick_Inst.Brick_Inst"))))

(fn SpawnTrap
  (params (Location :type Vector))
  (if (not (Variables|Default|GetOriginRoom))
    (if (not (Variables|Default|GetisShop))
      (LocalVariables|SetTrapLocation Location)
      (if (Variables|Default|GetHallway)
        (return false false)
        (else
          (bind _output_get (Variables|Default|SetCurrTrap (Utilities|GetClass (.OutItem (Utilities|Array|Random (Variables|Default|GetTrapArray))))))
          (if (== (Math|Random|RandomIntegerinRange 1 7) 1)
            (if (== (Variables|Default|GetCurrTrap) "/Game/Code/Objects/Traps/BP_PitfallTrap.BP_PitfallTrap_C")
              (bind _returnvalue (Game|SpawnActorfromClass _output_get (Math|Transform|MakeTransform "0, 0, 0" "0, 0, 0" "1.000000,1.000000,1.000000") "Undefined" "MultiplyWithRoot" 0 0))
              (bind _output_get_2 (LocalVariables|SetTrap _returnvalue))
              (Transformation|AttachActorToActor _output_get_2 self "None" "KeepRelative" "KeepRelative" "KeepRelative" true)
              (Transformation|SetActorRelativeLocation (LocalVariables|GetTrap) (LocalVariables|GetTrapLocation))
              (return (== (Variables|Default|GetCurrTrap) "/Game/Code/Objects/Traps/BP_PitfallTrap.BP_PitfallTrap_C") true)
              (else
                (bind _returnvalue_2 (Game|SpawnActorfromClass _output_get (Math|Transform|MakeTransform "0, 0, 0" "0, 0, 0" "1.000000,1.000000,1.000000") "Undefined" "MultiplyWithRoot" 0 0))
                (bind _output_get_3 (LocalVariables|SetTrap _returnvalue_2))
                (Transformation|AttachActorToActor _output_get_3 self "None" "KeepRelative" "KeepRelative" "KeepRelative" true)
                (if (== (Variables|Default|GetCurrTrap) "/Game/Code/Objects/Traps/BP_PendulumOfDeath.BP_PendulumOfDeath_C")
                  (Transformation|SetActorRelativeLocation (LocalVariables|GetTrap) (- (LocalVariables|GetTrapLocation) "-100.000000,-100.000000,-50.000000"))
                  (return false true)
                  (elif (== (Variables|Default|GetCurrTrap) "/Game/Code/Objects/Traps/BP_DartTrap.BP_DartTrap_C")
                    (Transformation|SetActorRelativeLocation (LocalVariables|GetTrap) (- (LocalVariables|GetTrapLocation) "0.000000,-100.000000,0.000000"))
                    (return false true)
                    (elif (== (Variables|Default|GetCurrTrap) "/Game/Code/Objects/Traps/BP_SpikeWheel.BP_SpikeWheel_C")
                      (Transformation|SetActorRelativeLocation (LocalVariables|GetTrap) (- (LocalVariables|GetTrapLocation) "-100.000000,-40.000000,0.000000"))
                      (return false true)
                      (elif (== (Variables|Default|GetCurrTrap) "/Game/Code/Objects/Traps/BP_BoulderWithPressurePlate.BP_BoulderWithPressurePlate_C")
                        (Transformation|SetActorRelativeLocation (LocalVariables|GetTrap) (- (LocalVariables|GetTrapLocation) "-100.000000,-100.000000,0.000000"))
                        (return false true)))))))
            (else
              (return false false))))))))

(fn SpawnAi
  (params (Location :type Vector))
  (if (not (Variables|Default|GetHallway))
    (if (not (Variables|Default|GetOriginRoom))
      (if (not (Variables|Default|GetisShop))
        (LocalVariables|SetSpawnLoc Location)
        (if (== (Math|Random|RandomIntegerinRange 0 15) 10)
          (bind _returnvalue (Game|SpawnActorfromClass "/Game/Code/AI/Variants/BP_NPC_WanderChase.BP_NPC_WanderChase_C" (Math|Transform|MakeTransform "1000.000000,1000.000000,1000.000000" "0, 0, 0" "1.000000,1.000000,1.000000") "Undefined" "MultiplyWithRoot" 0 0))
          (Transformation|AttachActorToActor _returnvalue self "None" "KeepRelative" "KeepRelative" "KeepRelative" true)
          (Transformation|SetActorRelativeLocation _returnvalue (+ (LocalVariables|GetSpawnLoc) "100.000000,100.000000,44.000000"))
          (return)
          (else
            (return)))))))

(fn SpawnShop
  (params (SpawnTransform_Location :type Vector))
  (Utilities|FlowControl|DoOnce false
    (:Completed
      (bind _returnvalue (Game|SpawnActorfromClass "/Game/Code/Shop/BP_5hop.BP_5hop_C" (Math|Transform|MakeTransform SpawnTransform_Location "0, 0, 0" "1.000000,1.000000,1.000000") "Undefined" "MultiplyWithRoot" 0 0))
      (Transformation|AttachActorToActor _returnvalue self "None" "KeepRelative" "KeepRelative" "KeepRelative" true)
      (if (> (Variables|Default|GetEnterShift) 0)
        (Transformation|SetRelativeLocation (Variables|/Script/Engine.Actor|GetRootComponent _returnvalue) (Math|Vector|MakeVector (Math|Conversions|ToFloat(Integer) (/ (* (Variables|Default|GetFloorTilesX) 200) 2)) (Math|Conversions|ToFloat(Integer) (+ (/ (* (Variables|Default|GetFloorTilesY) 200) 2) (* (Variables|Default|GetEnterShift) -200))) 0.0) false false)
        (Variables|/Game/Code/Gamemodes/GM_Roguelike.GM_Roguelike_C|SetshopSpawned (Variables|Default|GetGameMode) true)
        (return)
        (else
          (Transformation|SetRelativeLocation (Variables|/Script/Engine.Actor|GetRootComponent _returnvalue) (Math|Vector|MakeVector (Math|Conversions|ToFloat(Integer) (/ (* (Variables|Default|GetFloorTilesX) 200) 2)) (Math|Conversions|ToFloat(Integer) (/ (* (Variables|Default|GetFloorTilesY) 200) 2)) 0.0) false false)
          (Variables|/Game/Code/Gamemodes/GM_Roguelike.GM_Roguelike_C|SetshopSpawned (Variables|Default|GetGameMode) true)
          (return))))))

(fn SpawnProps
  (params (Location :type Vector))
  (if (not (Variables|Default|GetTrapped))
    (if (not (Variables|Default|GetHallway))
      (if (not (Variables|Default|GetOriginRoom))
        (if (not (Variables|Default|GetisShop))
          (LocalVariables|SetCurrProp (Utilities|GetClass (.OutItem (Utilities|Array|Random (Variables|Default|GetPropArray)))))
          (if (== (Math|Random|RandomIntegerinRange 1 6) 6)
            (bind _returnvalue (Game|SpawnActorfromClass (LocalVariables|GetCurrProp) (Math|Transform|MakeTransform "1.000000,1.000000,1.000000" "0, 0, 0" "1.000000,1.000000,1.000000") "Undefined" "MultiplyWithRoot" 0 0))
            (Transformation|AttachActorToActor _returnvalue self "None" "KeepRelative" "KeepRelative" "KeepRelative" true)
            (Transformation|SetActorRelativeLocation _returnvalue Location)
            (return)
            (else
              (return))))))))