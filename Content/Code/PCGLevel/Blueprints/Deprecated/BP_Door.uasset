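; Deprecated procedural-level door that swings open or closed on Activate and, while CanRoom is set, spawns a BP_Room beyond it on opening.
; A seeded random stream picks a size limit, then a debug-drawn line trace probes along the door's right vector.
; A hit door (its room generation disabled) or wall collision (index removed) yields a one-tile-wide hallway sized to the hit distance; no hit yields a random room.
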(event Custom|GenerateNewRoom
  (params (RoomTileY :type Integer) (RoomTileX :type Integer) (MaxDoors :type Integer) (Shift :type Integer) (Hallway :type Boolean))
  (Game|SpawnActorfromClass "/Game/Code/PCGLevel/Blueprints/Deprecated/BP_Room.BP_Room_C" (Math|Transform|MakeTransform (+ (Transformation|GetActorLocation) (* (Transformation|GetActorForwardVector) 4e+02)) (Math|Rotator|CombineRotators (Transformation|GetActorRotation) "0.000000,90.000000,0.000000") "1.000000,1.000000,1.000000") "Undefined" "MultiplyWithRoot" 0 RoomTileY RoomTileX MaxDoors Shift Hallway 0))

(event Custom|AddAdditional
  (bind _returnvalue (Transformation|GetActorTransform))
  (bind _doorstream (Variables|Default|GetDoorStream))
  (bind _roomsizelimit (Variables|Default|GetRoomSizeLimit))
  (bind _returnvalue_2 (Math|Transform|TransformLocation _returnvalue "200.000000,10.000000,200.000000"))
  (bind _returnvalue_3 (Math|Random|RandomIntegerinRangefromStream _doorstream 3 _roomsizelimit))
  (bind (_outhit _returnvalue_4) (Collision|LineTraceByChannel _returnvalue_2 (+ _returnvalue_2 (* (Transformation|GetActorRightVector) (* (Variables|Default|GetRoomSizeLimit) (Variables|Default|GetTileSize)))) "TraceTypeQuery1" false 0 "Persistent"))
  (if _returnvalue_4
    (switch string (Utilities|GetClassDisplayName (Utilities|GetClass (.HitActor (Collision|BreakHitResult _outhit))))
      (:BP_Door_C
        (bind _asbp_door (Utilities|Casting|CastToBP_Door (.HitActor (Collision|BreakHitResult _outhit))))
        (Variables|BP_Door_C|SetCanRoom _asbp_door false))
      (:BP_WallCollision_C
        (bind _asbp_wall_collision (Utilities|Casting|CastToBP_WallCollision (.HitActor (Collision|BreakHitResult _outhit))))
        (Default|RemoveIndex _asbp_wall_collision)))
    (CallFunction|GenerateNewRoom 1 (Math|Float|Round (/ (.Distance (Collision|BreakHitResult _outhit)) (Variables|Default|GetTileSize))) (Math|Random|RandomIntegerinRangefromStream (Variables|Default|GetDoorStream) 1 5) 0 true)
    (else
      (CallFunction|GenerateNewRoom _returnvalue_3 _returnvalue_3 (Math|Random|RandomIntegerinRangefromStream (Variables|Default|GetDoorStream) 2 8) 0 false))))

(event Custom|OldGenerateNewRoom
  (Variables|Default|SetRandomRoomX (Math|Random|RandomIntegerinRange 3 8))
  (Variables|Default|SetRandomRoomY (Math|Random|RandomIntegerinRange 3 8))
  (Variables|Default|SetRandomDoorValue (Math|Random|RandomIntegerinRange 4 6))
  (Game|SpawnActorfromClass "/Game/Code/PCGLevel/Blueprints/Deprecated/BP_Room.BP_Room_C" (Math|Transform|MakeTransform (+ (Transformation|GetActorLocation) (* (Transformation|GetActorForwardVector) 4e+02)) (Math|Rotator|CombineRotators (Transformation|GetActorRotation) "0.000000,90.000000,0.000000") "1.000000,1.000000,1.000000") "Undefined" "MultiplyWithRoot" 0 (Variables|Default|GetRandomRoomY) (Variables|Default|GetRandomRoomX) (Variables|Default|GetRandomDoorValue) 0 false 0))

(event EventBeginPlay
  (Variables|Default|SetDoorStream (Math|Random|MakeRandomStream (Variables|Default|GetSeed))))

(event EventActivate
  (if (Variables|Default|GetClosed)
    (Variables|Default|SetClosed false)
    (Utilities|FlowControl|Sequence
      (:then_0
        (if (Variables|Default|GetCanRoom)
          (Variables|Default|SetCanRoom false)
          (bind _output_get (Variables|Default|SetRoomSizeLimit (Math|Random|RandomIntegerinRangefromStream (Variables|Default|GetDoorStream) 3 10)))
          (bind _output_get_2 (Variables|Default|SetLeftLimit _output_get))
          (Variables|Default|SetRightLimit _output_get_2)
          (CallFunction|AddAdditional)))
      (:then_1
        (bind _doortrack (Timeline|DoorSwingTimeline Play)
          (:Update
            (Transformation|SetRelativeRotation (Variables|Default|GetHinge) (Math|Rotator|MakeRotator 0.0 0.0 _doortrack) false false)))))
    (else
      (Variables|Default|SetClosed true)
      (Timeline|DoorSwingTimeline Reverse))))

(fn ConstructionScript)