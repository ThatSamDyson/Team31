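; Game mode for Joblins that adds a local player at startup and spawns a pawn for each player.
; BeginPlay creates the extra player with its own controller, waits briefly, then caches the level's PlayerStart actors.
; SpawnPlayers spawns the default pawn class at the PlayerStart matching each player index and has that player's controller possess it, without checking that enough starts exist.
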(event Custom|Spawn%20Players
  (bind _returnvalue (Class|GameModeBase|GetNumPlayers))
  (for _index (range 0 (- _returnvalue 1))
    (bind _returnvalue_2 (Game|SpawnActorfromClass (Variables|Default|GetDefaultPawnClass) (Transformation|GetActorTransform (Utilities|Array|Get(acopy) (Variables|Default|GetPlayer%20Starts) _index)) "Undefined" "MultiplyWithRoot" 0 0))
    (Pawn|Possess (Game|GetPlayerController _index) _returnvalue_2)))

(event EventBeginPlay
  (Class|GameplayStatics|CreatePlayer -1)
  (Utilities|FlowControl|Delay 1.0)
  (bind _outactors (Actor|GetAllActorsOfClass "/Script/Engine.PlayerStart"))
  (Variables|Default|SetPlayer%20Starts _outactors)
  (CallFunction|SpawnPlayers))

(fn ConstructionScript)