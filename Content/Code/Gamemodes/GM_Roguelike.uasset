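; GM_Roguelike is the game mode for the roguelike mode, setting up the player and tracking elapsed time.
; BeginPlay unpauses with game-only input and a visible cursor, then loads slot1 or creates a BP_GameSave, storing only a newly created save.
; It spawns CH_Roguelike at a fixed location and possesses it with the player controller.
; A one-second Delay on Tick drives the Seconds and Minutes counters.
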(event EventBeginPlay
  (bind _returnvalue (Game|GetPlayerController 0))
  (Input|SetInputModeGameOnly _returnvalue false)
  (Game|SetGamePaused false)
  (Variables|/Script/Engine.PlayerController|SetbShowMouseCursor _returnvalue true)
  (bind _returnvalue_2 (SaveGame|DoesSaveGameExist "slot1"))
  (if _returnvalue_2
    (SaveGame|LoadGamefromSlot "slot1")
    (else
      (bind _returnvalue_3 (SaveGame|CreateSaveGameObject "/Game/Code/Savegame/BP_GameSave.BP_GameSave_C"))
      (Variables|Default|SetSaveGame _returnvalue_3)))
  (bind _returnvalue_4 (Game|SpawnActorfromClass "/Game/Code/Character/CharacterBlueprints/CH_Roguelike.CH_Roguelike_C" (Math|Transform|MakeTransform "-60.000000,20.000000,92.000000" "0, 0, 0" "1.000000,1.000000,1.000000") "Undefined" "MultiplyWithRoot" 0 0))
  (Variables|Default|SetPlayerCharacter _returnvalue_4)
  (Pawn|Possess (Game|GetPlayerController 0) _returnvalue_4))

(event EventTick
  (params (DeltaSeconds :type Float%20%28single-precision%29))
  (Utilities|FlowControl|Delay 1.0)
  (Variables|Default|SetSeconds (+ (Variables|Default|GetSeconds) 1.0))
  (if (> (Variables|Default|GetSeconds) 59.0)
    (Variables|Default|SetMinutes (+ (Variables|Default|GetMinutes) 1.0))
    (Variables|Default|SetSeconds 0.0)))

(fn ConstructionScript)