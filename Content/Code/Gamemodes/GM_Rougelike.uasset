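; GM_Rougelike is a game mode Blueprint that sets up the player and HUD for the roguelike mode.
; On BeginPlay it spawns a CH_Rougelike character at a fixed location and has the first player controller possess it.
; It then creates WBP_HUD, passes it the character's health and money once with the two values crossed between inputs, and adds it to the viewport.
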(event EventBeginPlay
  (bind _returnvalue (Game|SpawnActorfromClass "/Game/Code/Character/CharacterBlueprints/CH_Rougelike.CH_Rougelike_C" (Math|Transform|MakeTransform "-60.000000,20.000000,92.000000" "0, 0, 0" "1.000000,1.000000,1.000000") "Undefined" "MultiplyWithRoot" 0 0))
  (Variables|Default|SetPlayerCharacter _returnvalue)
  (Pawn|Possess (Game|GetPlayerController 0) _returnvalue)
  (bind _returnvalue_2 (UserInterface|CreateWidget "/Game/Code/Widgets/WBP_HUD.WBP_HUD_C"))
  (bind _output_get (Variables|Default|SetHUD _returnvalue_2))
  (Default|GetMoneyandHealth _output_get (Variables|/Game/Code/Character/CharacterBlueprints/CH_Rougelike.CH_Rougelike_C|GetplayerHealth (Variables|Default|GetPlayerCharacter)) (Variables|/Game/Code/Character/CharacterBlueprints/CH_Rougelike.CH_Rougelike_C|GetplayerMoney (Variables|Default|GetPlayerCharacter)))
  (UserInterface|Viewport|AddtoViewport (Variables|Default|GetHUD) 0))

(event EventTick
  (params (DeltaSeconds :type Float%20%28single-precision%29)))

(fn ConstructionScript)