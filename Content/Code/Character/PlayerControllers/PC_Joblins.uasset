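; PC_Joblins is a player controller that handles Enhanced Input for the Joblins character.
; On BeginPlay it waits two seconds, as a noted workaround for a UE 5.2 bug, then adds the IMC_Joblins mapping context, printing an error if the input subsystem is invalid.
; Triggered move-right, jump and climb actions are forwarded to the controlled pawn as messages, leaving the response to the pawn.
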(event Input|EnhancedActionEvents|EnhancedInputActionIA_Climb
  (params (ActionValue :type Boolean) (ElapsedSeconds :type Float%20%28double-precision%29) (TriggeredSeconds :type Float%20%28double-precision%29) (InputAction :type Input%20Action%20Object%20Reference :default "/Game/Code/Input/IA_Climb.IA_Climb"))
  (:Triggered
    (Class|BIInputs|IAClimb(Message) (Pawn|GetControlledPawn) ActionValue "None")))

(event Input|EnhancedActionEvents|EnhancedInputActionIA_MoveRight
  (params (ActionValue :type Float%20%28double-precision%29) (ElapsedSeconds :type Float%20%28double-precision%29) (TriggeredSeconds :type Float%20%28double-precision%29) (InputAction :type Input%20Action%20Object%20Reference :default "/Game/Code/Input/IA_MoveRight.IA_MoveRight"))
  ;[1 1 1] Enhanced Input Action
  (:Triggered
    (Class|BIInputs|IAMoveRight(Message) (Pawn|GetControlledPawn) ActionValue "Triggered")))

(event Input|EnhancedActionEvents|EnhancedInputActionIA_Jump
  (params (ActionValue :type Boolean) (ElapsedSeconds :type Float%20%28double-precision%29) (TriggeredSeconds :type Float%20%28double-precision%29) (InputAction :type Input%20Action%20Object%20Reference :default "/Game/Code/Input/IA_Jump.IA_Jump"))
  ;[1 1 1] Enhanced Input Action
  (:Triggered
    (Class|BIInputs|IAJump(Message) (Pawn|GetControlledPawn) ActionValue "None")))

(event EventBeginPlay
  (bind _self self)
  (bind _returnvalue (PlayerController|LocalPlayerSubsystems|GetEnhancedInputLocalPlayerSubsystem _self))
  ;[1 1 1] Event Begin Play
  (Utilities|FlowControl|Delay 2.0) ; This is a Bodge Fix for UE5.2 being Broken
  (Utilities|IsValid _returnvalue
    (:Is%20Valid
      (Input|AddMappingContext _returnvalue "/Game/Code/Input/IMC_Joblins.IMC_Joblins" 0 "(bIgnoreAllPressedKeysUntilRelease=True,bForceImmediately=False)"))
    (:Is%20Not%20Valid
      (Development|PrintString "Can not Get Input System" true true "(R=1.000000,G=0.000000,B=0.000000,A=1.000000)" 5.0))))

(fn ConstructionScript)