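; Player controller for the roguelike mode that sets up Enhanced Input and relays it to the possessed pawn.
; On BeginPlay it adds the IMC_Rougelike mapping context, printing an error if the input subsystem is unavailable.
; Triggered move forward, move right and turn actions are forwarded to the controlled pawn as interface messages, so the pawn implements the actual movement.
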(event Input|EnhancedActionEvents|EnhancedInputActionIA_MoveForward
  (params (ActionValue :type Float%20%28double-precision%29) (ElapsedSeconds :type Float%20%28double-precision%29) (TriggeredSeconds :type Float%20%28double-precision%29) (InputAction :type Input%20Action%20Object%20Reference :default "/Game/Code/Input/IA_MoveForward.IA_MoveForward"))
  ;[1 1 1] Enhanced Input Action
  (:Triggered
    (Class|BIInputs|IAMoveForward(Message) (Pawn|GetControlledPawn) ActionValue "Triggered")))

(event Input|EnhancedActionEvents|EnhancedInputActionIA_MoveRight
  (params (ActionValue :type Float%20%28double-precision%29) (ElapsedSeconds :type Float%20%28double-precision%29) (TriggeredSeconds :type Float%20%28double-precision%29) (InputAction :type Input%20Action%20Object%20Reference :default "/Game/Code/Input/IA_MoveRight.IA_MoveRight"))
  ;[1 1 1] Enhanced Input Action
  (:Triggered
    (Class|BIInputs|IAMoveRight(Message) (Pawn|GetControlledPawn) ActionValue "Triggered")))

(event Input|EnhancedActionEvents|EnhancedInputActionIA_Turn
  (params (ActionValue :type Float%20%28double-precision%29) (ElapsedSeconds :type Float%20%28double-precision%29) (TriggeredSeconds :type Float%20%28double-precision%29) (InputAction :type Input%20Action%20Object%20Reference :default "/Game/Code/Input/IA_Turn.IA_Turn"))
  ;[1 1 1] Enhanced Input Action
  (:Triggered
    (Class|BIInputs|IATurn(Message) (Pawn|GetControlledPawn) ActionValue "Triggered")))

(event EventBeginPlay
  (bind _self self)
  (bind _returnvalue (PlayerController|LocalPlayerSubsystems|GetEnhancedInputLocalPlayerSubsystem _self))
  ;[1 1 1] Event Begin Play
  (Utilities|IsValid _returnvalue
    (:Is%20Valid
      (Input|AddMappingContext _returnvalue "/Game/Code/Input/IMC_Rougelike.IMC_Rougelike" 0 "(bIgnoreAllPressedKeysUntilRelease=True,bForceImmediately=False)"))
    (:Is%20Not%20Valid
      (Development|PrintString "Can not Get Input System" true true "(R=1.000000,G=0.000000,B=0.000000,A=1.000000)" 5.0))))

(fn ConstructionScript)