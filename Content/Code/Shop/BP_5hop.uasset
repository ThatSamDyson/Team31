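; BP_5hop is a shop that opens its UI when activated and pauses the game.
; Activate creates a WBP_Shop widget, adds it to the viewport and initializes it with the player character, itself, the available items and the current shop items.
; It then hands input to the widget in UI-only mode and shows the mouse cursor; closing and unpausing are not handled here.
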(event EventActivate
  (bind _returnvalue (Game|GetPlayerController 0))
  (bind _returnvalue_2 (UserInterface|CreateWidget "/Game/Code/Shop/WBP_Shop.WBP_Shop_C" _returnvalue))
  (bind _output_get (Variables|Default|SetShopUIRef _returnvalue_2))
  (UserInterface|Viewport|AddtoViewport _output_get 0)
  (Default|Init _output_get (Variables|Default|GetPlayerCharacterRef) self (Variables|Default|GetAvailableItems) (Variables|Default|GetShopItems))
  (Input|SetInputModeUIOnly _returnvalue _output_get "DoNotLock" false)
  (Variables|/Script/Engine.PlayerController|SetbShowMouseCursor _returnvalue true)
  (Game|SetGamePaused true))

(fn ConstructionScript)