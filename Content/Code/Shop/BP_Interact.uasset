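; BP_Interact is a shop trigger that opens the shop UI when a character enters its Box volume.
; On overlap by a BI_Character implementer, it creates WBP_Shop if no reference is held, shows it with UI-only input and mouse cursor, and pauses the game.
; Any end overlap only clears the widget reference; removing the widget, restoring input and unpausing are not handled here.
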(event OnComponentBeginOverlap(Box)
  (params (OverlappedComponent :type Primitive%20Component%20Object%20Reference) (OtherActor :type Actor%20Object%20Reference) (OtherComp :type Primitive%20Component%20Object%20Reference) (OtherBodyIndex :type Integer) (bFromSweep :type Boolean) (SweepResult :type Hit%20Result%20Structure%20%28by%20ref%29))
  (bind _returnvalue (Game|GetPlayerController 0))
  (if (Utilities|DoesObjectImplementInterface OtherActor "/Game/Code/Interfaces/BI_Character.BI_Character_C")
    (if (== (Variables|Default|GetShopUI) 0)
      (bind _returnvalue_2 (UserInterface|CreateWidget "/Game/Code/Shop/WBP_Shop.WBP_Shop_C" _returnvalue))
      (bind _output_get (Variables|Default|SetShopUI _returnvalue_2))
      (UserInterface|Viewport|AddtoViewport _output_get 0)
      (Input|SetInputModeUIOnly _returnvalue _output_get "DoNotLock" false)
      (Variables|/Script/Engine.PlayerController|SetbShowMouseCursor _returnvalue true)
      (Game|SetGamePaused true))))

(event OnComponentEndOverlap(Box)
  (params (OverlappedComponent :type Primitive%20Component%20Object%20Reference) (OtherActor :type Actor%20Object%20Reference) (OtherComp :type Primitive%20Component%20Object%20Reference) (OtherBodyIndex :type Integer))
  (if (!= (Variables|Default|GetShopUI) 0)
    (Variables|Default|SetShopUI 0)))

(fn ConstructionScript)