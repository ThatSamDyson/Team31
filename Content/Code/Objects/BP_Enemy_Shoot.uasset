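; Enemy shot actor that damages the player on overlap and destroys itself a few seconds after BeginPlay.
; Its Box overlap checks whether the other actor implements BI_Character and prints debug strings for each outcome.
; On a match it applies fixed damage to the CH_Roguelike found by GetActorOfClass, not to the overlapping actor itself.
; A hit does not destroy the shot.
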(event OnComponentBeginOverlap(Box)
  (params (OverlappedComponent :type Primitive%20Component%20Object%20Reference) (OtherActor :type Actor%20Object%20Reference) (OtherComp :type Primitive%20Component%20Object%20Reference) (OtherBodyIndex :type Integer) (bFromSweep :type Boolean) (SweepResult :type Hit%20Result%20Structure%20%28by%20ref%29))
  (Development|PrintString "Collide")
  (if (Utilities|DoesObjectImplementInterface OtherActor "/Game/Code/Interfaces/BI_Character.BI_Character_C")
    (Development|PrintString "Collide Player")
    (bind _returnvalue (Actor|GetActorOfClass "/Game/Code/Character/CharacterBlueprints/CH_Roguelike.CH_Roguelike_C"))
    (bind _output_get (Variables|Default|SetColliding%20Player _returnvalue))
    (Default|TakeDamage _output_get 1e+01)
    (else
      (Development|PrintString "Collide with not Player"))))

(event EventBeginPlay
  (Utilities|FlowControl|Delay 3.0)
  (Actor|DestroyActor))

(fn ConstructionScript)