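; Pitfall trap with a hinged trapdoor over a spike death zone.
; BoxTrigger overlaps by BI_Health actors play a timeline that drives both hinges' pitch, and ending the overlap reverses it.
; BeginPlay derives open angles from the closed hinge rotations.
; In DeathZone, a BI_Character overlap calls KillPlayer on the CH_Roguelike found by GetActorOfClass, while other actors trigger an ApplyDamage call.
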(event OnComponentBeginOverlap(BoxTrigger)
  (params (OverlappedComponent :type Primitive%20Component%20Object%20Reference) (OtherActor :type Actor%20Object%20Reference) (OtherComp :type Primitive%20Component%20Object%20Reference) (OtherBodyIndex :type Integer) (bFromSweep :type Boolean) (SweepResult :type Hit%20Result%20Structure%20%28by%20ref%29))
  ;[1 1 1] Opening and closing of the trapdoor
  (if (Utilities|DoesObjectImplementInterface OtherActor "/Game/Code/Interfaces/BI_Health.BI_Health_C")
    (Components|Timeline|SetPlayRate (Variables|Default|GetTL_TrapDoor) (Variables|Default|GetTrapPlaybackRate))
    (bind _trapdoor (Timeline|TL_TrapDoor Play)
      (:Update
        (Transformation|SetRelativeRotation (Variables|Default|GetBottomHinge) (Math|Rotator|MakeRotator 0.0 (Math|Float|Lerp (Variables|Default|GetLHDoorClose) (Variables|Default|GetLHDoorOpen) _trapdoor) 0.0) false false)
        (Transformation|SetRelativeRotation (Variables|Default|GetTopHinge) (Math|Rotator|MakeRotator 0.0 (Math|Float|Lerp _trapdoor (Variables|Default|GetRHDoorClose) (Variables|Default|GetRHDoorOpen)) 0.0) false false)))))

(event OnComponentEndOverlap(BoxTrigger)
  (params (OverlappedComponent :type Primitive%20Component%20Object%20Reference) (OtherActor :type Actor%20Object%20Reference) (OtherComp :type Primitive%20Component%20Object%20Reference) (OtherBodyIndex :type Integer))
  ;[1 1 1] Opening and closing of the trapdoor
  (if (Utilities|DoesObjectImplementInterface OtherActor "/Game/Code/Interfaces/BI_Health.BI_Health_C")
    (bind _trapdoor (Timeline|TL_TrapDoor Reverse)
      (:Update
        (Transformation|SetRelativeRotation (Variables|Default|GetBottomHinge) (Math|Rotator|MakeRotator 0.0 (Math|Float|Lerp (Variables|Default|GetLHDoorClose) (Variables|Default|GetLHDoorOpen) _trapdoor) 0.0) false false)
        (Transformation|SetRelativeRotation (Variables|Default|GetTopHinge) (Math|Rotator|MakeRotator 0.0 (Math|Float|Lerp _trapdoor (Variables|Default|GetRHDoorClose) (Variables|Default|GetRHDoorOpen)) 0.0) false false)))))

(event OnComponentBeginOverlap(DeathZone)
  (params (OverlappedComponent :type Primitive%20Component%20Object%20Reference) (OtherActor :type Actor%20Object%20Reference) (OtherComp :type Primitive%20Component%20Object%20Reference) (OtherBodyIndex :type Integer) (bFromSweep :type Boolean) (SweepResult :type Hit%20Result%20Structure%20%28by%20ref%29))
  ;[1 1 1] Killing the player when touching the spikes
  (if (Utilities|DoesObjectImplementInterface OtherActor "/Game/Code/Interfaces/BI_Character.BI_Character_C")
    (bind _returnvalue (Actor|GetActorOfClass "/Game/Code/Character/CharacterBlueprints/CH_Roguelike.CH_Roguelike_C"))
    (Default|KillPlayer _returnvalue)
    (else
      (Game|Damage|ApplyDamage 0 0.0 0 0 "/Script/Engine.DamageType"))))

(event EventBeginPlay
  ;[1 1 1] Sets rotations for trap door on Begin Play
  (bind _output_get (Variables|Default|SetLHDoorClose (.pitch (Transformation|GetWorldRotation (Variables|Default|GetBottomHinge)))))
  (bind _output_get_2 (Variables|Default|SetRHDoorClose (.pitch (Transformation|GetWorldRotation (Variables|Default|GetTopHinge)))))
  (Variables|Default|SetLHDoorOpen (+ _output_get 9e+01))
  (Variables|Default|SetRHDoorOpen (+ _output_get_2 9e+01)))

(fn ConstructionScript)