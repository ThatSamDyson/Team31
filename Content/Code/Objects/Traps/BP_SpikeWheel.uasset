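; Spike wheel trap that spins while sliding along the actor's right axis and damages what it touches.
; A RotatingMovement component spins Outer, while a timeline at PlayRate lerps SpikeWheel from its start position to a fixed sideways offset.
; Box overlaps with BI_Character implementers damage the CH_Roguelike found by class lookup, not the overlapping actor.
; Other overlaps call ApplyDamage with no target wired.
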(event OnComponentBeginOverlap(Box)
  (params (OverlappedComponent :type Primitive%20Component%20Object%20Reference) (OtherActor :type Actor%20Object%20Reference) (OtherComp :type Primitive%20Component%20Object%20Reference) (OtherBodyIndex :type Integer) (bFromSweep :type Boolean) (SweepResult :type Hit%20Result%20Structure%20%28by%20ref%29))
  ;[1 1 1] Apply damage to the player if it hits them
  (if (Utilities|DoesObjectImplementInterface OtherActor "/Game/Code/Interfaces/BI_Character.BI_Character_C")
    (bind _returnvalue (Actor|GetActorOfClass "/Game/Code/Character/CharacterBlueprints/CH_Roguelike.CH_Roguelike_C"))
    (Default|TakeDamage _returnvalue (Variables|Default|GetBladeDamage))
    (else
      (Game|Damage|ApplyDamage 0 (Variables|Default|GetBladeDamage) 0 0))))

(event EventBeginPlay
  (Utilities|FlowControl|Delay 0.1)
  (Variables|Default|SetStartPosition (Transformation|GetWorldLocation (Variables|Default|GetSpikeWheel)))
  (Components|Timeline|SetPlayRate (Variables|Default|GetTL_Movement) (Variables|Default|GetPlayRate))
  (Components|Movement|SetUpdatedComponent (Variables|Default|GetRotatingMovement) (Variables|Default|GetOuter))
  (Variables|/Script/Engine.RotatingMovementComponent|SetRotationRate (Variables|Default|GetRotatingMovement) "0.000000,0.000000,180.000000")
  (Variables|Default|SetEndPosition (* (Transformation|GetActorRightVector) 1.2e+02))
  (bind _alpha (Timeline|TL_Movement Play)
    (:Update
      (Transformation|SetWorldLocation (Variables|Default|GetSpikeWheel) (Math|Vector|Lerp(Vector) (Variables|Default|GetStartPosition) (+ (Variables|Default|GetStartPosition) (Variables|Default|GetEndPosition)) _alpha) false false))))

(fn ConstructionScript)