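; Trap actor that moves a damaging spike wheel blade along a spline track, filed under NotInUse.
; On BeginPlay it copies the local points of a randomly chosen preset actor's spline into its own spline.
; It then spawns a BP_SpikeWheel at the first point, passes on damage and zeroes its rotating movement.
; A timeline, rate-scaled by track speed, sets the blade's location and rotation by distance along the spline.
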(event Custom|MoveBlade
  (bind _blade (Variables|Default|GetBlade))
  (bind _spline (Variables|Default|GetSpline))
  (bind _spline_2 (Variables|Default|GetSpline))
  ;[1 1 1] Move blade along spline
  (bind _blademovement (Timeline|BladeTimeline Play)
    (:Update
      (Transformation|SetActorLocation _blade (Spline|GetLocationatDistanceAlongSpline _spline_2 (Math|Float|Lerp 0.0 (Spline|GetDistanceAlongSplineatSplinePoint _spline (- (Spline|GetNumberOfSplinePoints _spline) 1)) _blademovement) "World") false false)
      (Transformation|SetActorRotation _blade (Spline|GetRotationatDistanceAlongSpline _spline_2 (Math|Float|Lerp 0.0 (Spline|GetDistanceAlongSplineatSplinePoint _spline (- (Spline|GetNumberOfSplinePoints _spline) 1)) _blademovement) "World")))))

(event Custom|SetSplinePoints
  ;[1 1 1] Chooses a random spline from the array and sets the positions for the blade to follow
  (Utilities|Array|Clear (Variables|Default|GetSplinePointPositions))
  (bind _output_get (Variables|Default|SetChosenSpline (Actor|GetComponentbyClass (.OutItem (Utilities|Array|Random (Variables|Default|GetSplinePresets))) "/Script/Engine.SplineComponent")))
  (Utilities|IsValid _output_get
    (:Is%20Valid
      (for _index (range 0 (- (Spline|GetNumberOfSplinePoints (Variables|Default|GetChosenSpline)) 1))
        (Utilities|Array|Add (Variables|Default|GetSplinePointPositions) (Spline|GetLocationatSplinePoint (Variables|Default|GetChosenSpline) _index "Local")))
      (Spline|SetSplinePoints (Variables|Default|GetSpline) (Variables|Default|GetSplinePointPositions) "Local" true))))

(event EventBeginPlay
  ;[1 1 1] Sets Spline points, play rate, spawns the blade and sets its default values.
  (CallFunction|SetSplinePoints)
  (Components|Timeline|SetPlayRate (Variables|Default|GetBladeTimeline) (Variables|Default|GetTrackMoveSpeed))
  (bind _returnvalue (Game|SpawnActorfromClass "/Game/Code/Objects/Traps/BP_SpikeWheel.BP_SpikeWheel_C" (Math|Conversions|ToTransform(Vector) (Spline|GetLocationatSplinePoint (Variables|Default|GetSpline) 0 "World")) "Undefined" "MultiplyWithRoot" 0 0))
  (bind _output_get (Variables|Default|SetBlade _returnvalue))
  (Variables|/Game/Code/Objects/Traps/BP_SpikeWheel.BP_SpikeWheel_C|SetBladeDamage _output_get (Variables|Default|GetDamage))
  (Variables|/Script/Engine.RotatingMovementComponent|SetRotationRate (Variables|/Game/Code/Objects/Traps/BP_SpikeWheel.BP_SpikeWheel_C|GetRotatingMovement _output_get) (Math|Rotator|MakeRotator 0.0 0.0 0.0))
  (CallFunction|MoveBlade))

(fn ConstructionScript)