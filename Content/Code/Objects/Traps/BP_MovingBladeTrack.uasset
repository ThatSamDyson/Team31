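; BP_MovingBladeTrack is a trap that spawns a BP_MovingBlade and moves it along a spline.
; BeginPlay places the blade at the first spline point, passes it damage and spin rate, and sets the timeline's play rate.
; The timeline's alpha maps to distance along the spline to position the blade.
; An unused SetSplinePoints event can copy a random preset's spline points onto the track.
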(event Custom|MoveBlade
  (bind _spline (Variables|Default|GetSpline))
  (bind _blademovement (Timeline|BladeTimeline Play)
    (:Update
      (Transformation|SetActorLocation (Variables|Default|GetBlade) (Spline|GetLocationatDistanceAlongSpline (Variables|Default|GetSpline) (Math|Float|Lerp 0.0 (Spline|GetDistanceAlongSplineatSplinePoint _spline (- (Spline|GetNumberOfSplinePoints _spline) 1)) _blademovement) "World") false false))))

(event Custom|SetSplinePoints
  (Utilities|Array|Clear (Variables|Default|GetSplinePointPositions))
  (bind _output_get (Variables|Default|SetChosenSpline (Actor|GetComponentbyClass (.OutItem (Utilities|Array|Random (Variables|Default|GetSplinePresets))) "/Script/Engine.SplineComponent")))
  (Utilities|IsValid _output_get
    (:Is%20Valid
      (for _index (range 0 (- (Spline|GetNumberOfSplinePoints (Variables|Default|GetChosenSpline)) 1))
        (Utilities|Array|Add (Variables|Default|GetSplinePointPositions) (Spline|GetLocationatSplinePoint (Variables|Default|GetChosenSpline) _index "Local")))
      (Spline|SetSplinePoints (Variables|Default|GetSpline) (Variables|Default|GetSplinePointPositions) "Local" true))))

(event EventBeginPlay
  (Components|Timeline|SetPlayRate (Variables|Default|GetBladeTimeline) (Variables|Default|GetTrackMoveSpeed))
  (bind _returnvalue (Game|SpawnActorfromClass "/Game/Code/Objects/Traps/BP_MovingBlade.BP_MovingBlade_C" (Math|Conversions|ToTransform(Vector) (Spline|GetLocationatSplinePoint (Variables|Default|GetSpline) 0 "World")) "Undefined" "MultiplyWithRoot" 0 0))
  (bind _output_get (Variables|Default|SetBlade _returnvalue))
  (Variables|/Game/Code/Objects/Traps/BP_MovingBlade.BP_MovingBlade_C|SetBladeDamage _output_get (Variables|Default|GetDamage))
  (Variables|/Script/Engine.RotatingMovementComponent|SetRotationRate (Variables|/Game/Code/Objects/Traps/BP_MovingBlade.BP_MovingBlade_C|GetRotatingMovement _output_get) (Math|Rotator|MakeRotator 0.0 0.0 (Variables|Default|GetRotationRate)))
  (CallFunction|MoveBlade))

(fn ConstructionScript)