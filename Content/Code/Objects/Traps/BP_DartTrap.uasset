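; Pressure-plate dart trap that rises from the ground and fires BP_Enemy_Shoot projectiles from its firing points when a BI_Health actor overlaps its trigger.
; A Timeline lerps the trap by a target offset from its cached start position, and firing waits until movement finishes.
; Continuous mode fires on a looping timer until overlap ends, while burst mode uses a delayed DoN loop, then lowers the trap.
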(event OnComponentBeginOverlap(Trigger)
  (params (OverlappedComponent :type Primitive%20Component%20Object%20Reference) (OtherActor :type Actor%20Object%20Reference) (OtherComp :type Primitive%20Component%20Object%20Reference) (OtherBodyIndex :type Integer) (bFromSweep :type Boolean) (SweepResult :type Hit%20Result%20Structure%20%28by%20ref%29))
  ;[1 1 1] Activates Trap if the preesure plate has been stood on
  (if (Utilities|DoesObjectImplementInterface OtherActor "/Game/Code/Interfaces/BI_Health.BI_Health_C")
    (CallFunction|TrapTriggered)))

(event OnComponentEndOverlap(Trigger)
  (params (OverlappedComponent :type Primitive%20Component%20Object%20Reference) (OtherActor :type Actor%20Object%20Reference) (OtherComp :type Primitive%20Component%20Object%20Reference) (OtherBodyIndex :type Integer))
  ;[1 1 1] Activates Trap if the preesure plate has been stood on
  (if (Utilities|DoesObjectImplementInterface OtherActor "/Game/Code/Interfaces/BI_Health.BI_Health_C")
    (if (Variables|Default|GetContinousFiring)
      (CallFunction|DeactivateTrap))))

(event Custom|AppearOrHide
  (bind _startposition (Variables|Default|GetStartPosition))
  ;[1 1 1] Trap is hidden in the ground. This rasies the trap when the pressure plate is activated and lowers it after it has finished shooting.
  (Variables|Default|SetHasFinishedMoving false)
  (if (Variables|Default|GetActive)
    (Variables|Default|SetActive false)
    (bind _alpha (Timeline|Timeline Reverse)
      (:Update
        (Transformation|SetWorldLocation (Variables|Default|GetDartTrap) (Math|Vector|Lerp(Vector) _startposition (+ _startposition (Variables|Default|GetTargetPosition)) _alpha) false false))
      (:Finished
        (Variables|Default|SetHasFinishedMoving true)))
    (else
      (Variables|Default|SetActive true)
      (Timeline|Timeline Play))))

(event Custom|TrapTriggered
  (bind _burstamount (Variables|Default|GetBurstAmount))
  ;[1 1 1] Trigger trap. Then check if it is already in activated/moving. Then execute correct functions
  (if (Variables|Default|GetHasSetStart)
    _
    (else
      (CallFunction|SetStartLocation)))
  (if (not (Variables|Default|GetActive))
    (CallFunction|AppearorHide)
    (if (Variables|Default|GetHasFinishedMoving) :!label _label
      (if (Variables|Default|GetContinousFiring)
        ;[1 1 1] Shoot as long as player is on pressure plate
        (CallFunction|Shoot)
        (bind _returnvalue (Utilities|Time|SetTimerbyEvent (delegate Custom|Shoot) (Variables|Default|GetTimeBetweenFiring) true))
        (Variables|Default|SetTrapTimer _returnvalue)
        (else
          ;[1 1 1] Shoot a burst when player steps on pressure plate
          (bind _counter (Utilities|FlowControl|DoN _burstamount :!label _label_2)
            (:Exit
              (if (< _counter _burstamount)
                (for _array_element (Variables|Default|GetFiringPoints)
                  (Game|SpawnActorfromClass "/Game/Code/Objects/BP_Enemy_Shoot.BP_Enemy_Shoot_C" (Math|Transform|MakeTransform (Transformation|GetWorldLocation _array_element) (Transformation|GetWorldRotation _array_element) "1.000000,1.000000,1.000000") "Undefined" "MultiplyWithRoot" 0 0))
                (Utilities|FlowControl|Delay (Variables|Default|GetTimeBetweenFiring))
                (goto _label_2)
                (else
                  (CallFunction|AppearorHide)
                  (goto _label_2 Reset)))))))
      (else
        (Utilities|FlowControl|Delay 0.2)
        (goto _label)))))

(event Custom|SetStartLocation
  ;[1 1 1] Add all firing points to array to make shooting easier
  (Variables|Default|SetStartPosition (Transformation|GetWorldLocation (Variables|Default|GetDartTrap)))
  (Utilities|Array|Add (Variables|Default|GetFiringPoints) (Variables|Default|GetFiringPoint1))
  (Variables|Default|SetHasSetStart true))

(event Custom|DeactivateTrap
  ;[1 1 1] Shoot as long as player is on pressure plate
  (Utilities|Time|ClearandInvalidateTimerbyHandle (Variables|Default|GetTrapTimer))
  (CallFunction|AppearorHide))

(event Custom|Shoot
  ;[1 1 1] Shoot as long as player is on pressure plate
  (for _array_element (Variables|Default|GetFiringPoints)
    (Game|SpawnActorfromClass "/Game/Code/Objects/BP_Enemy_Shoot.BP_Enemy_Shoot_C" (Math|Transform|MakeTransform (Transformation|GetWorldLocation _array_element) (Transformation|GetWorldRotation _array_element) "1.000000,1.000000,1.000000") "Undefined" "MultiplyWithRoot" 0 0)))

(fn ConstructionScript)