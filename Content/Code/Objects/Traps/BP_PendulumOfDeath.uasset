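; BP_PendulumOfDeath is a swinging pendulum trap that deals damage on overlap.
; On BeginPlay, a timeline at a configurable play rate lerps the RotationPoint's world roll between start and end rotations.
; When Box overlaps a BI_Character implementer, it calls TakeDamage on the CH_Roguelike found via GetActorOfClass, not on the overlapping actor.
; Other overlaps call generic ApplyDamage, with no damaged actor specified.
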(event OnComponentBeginOverlap(Box)
  (params (OverlappedComponent :type Primitive%20Component%20Object%20Reference) (OtherActor :type Actor%20Object%20Reference) (OtherComp :type Primitive%20Component%20Object%20Reference) (OtherBodyIndex :type Integer) (bFromSweep :type Boolean) (SweepResult :type Hit%20Result%20Structure%20%28by%20ref%29))
  ;[1 1 1] Apply Damage
  (if (Utilities|DoesObjectImplementInterface OtherActor "/Game/Code/Interfaces/BI_Character.BI_Character_C")
    (bind _returnvalue (Actor|GetActorOfClass "/Game/Code/Character/CharacterBlueprints/CH_Roguelike.CH_Roguelike_C"))
    (Default|TakeDamage _returnvalue (Variables|Default|GetDamage))
    (else
      (Game|Damage|ApplyDamage 0 (Variables|Default|GetDamage) 0 0))))

(event EventBeginPlay
  ;[1 1 1] Swing
  (Components|Timeline|SetPlayRate (Variables|Default|GetTL_SwingTimeline) (Variables|Default|GetPlayRate))
  (bind _alpha (Timeline|TL_SwingTimeline Play)
    (:Update
      (Transformation|SetWorldRotation (Variables|Default|GetRotationPoint) (Math|Rotator|Lerp(Rotator) (Math|Rotator|MakeRotator (Variables|Default|GetStartRotation) 0.0 0.0) (Math|Rotator|MakeRotator (Variables|Default|GetEndRotation) 0.0 0.0) _alpha) false false))))

(fn ConstructionScript)