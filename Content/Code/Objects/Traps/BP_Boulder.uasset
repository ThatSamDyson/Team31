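; BP_Boulder is a one-shot trap that rolls when an actor implementing BI_Health enters its trigger radius.
; It traces toward a flattened 2000-unit direction vector, used as a world position without adding the boulder's location, and targets any hit.
; A timeline lerps it there without sweeping, while a timer raises play rate to build speed.
; The unfinished fire variant only records trail points and draws debug circles; no damage is applied.
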(event OnComponentBeginOverlap(TriggerRadius)
  (params (OverlappedComponent :type Primitive%20Component%20Object%20Reference) (OtherActor :type Actor%20Object%20Reference) (OtherComp :type Primitive%20Component%20Object%20Reference) (OtherBodyIndex :type Integer) (bFromSweep :type Boolean) (SweepResult :type Hit%20Result%20Structure%20%28by%20ref%29))
  ;[1 1 1] When player or enemy walks within a radius of the boulder, it activates (could drop from ceiling). The vector of the boulder to the player is calculated then a line trace finds first thing it will hit. Then it will roll towards that
  (if (not (Variables|Default|GetActivated))
    (if (Utilities|DoesObjectImplementInterface OtherActor "/Game/Code/Interfaces/BI_Health.BI_Health_C")
      (Variables|Default|SetActivated true)
      (bind _output_get (Variables|Default|SetTargetPosition (* (* (Math|Vector|Normalize (- (Transformation|GetActorLocation OtherActor) (Transformation|GetActorLocation))) 2e+03) "1.000000,1.000000,0.000000")))
      (bind _outhit (Collision|LineTraceByChannel (Transformation|GetActorLocation) _output_get "TraceTypeQuery1" false 0 "Persistent"))
      (if (Math|Vector|VectorIsZero (.location _outhit))
        _
        (else
          (Variables|Default|SetTargetPosition (.location _outhit))))
      ;[1 1 1] Started working on leaving a trail of fire if it is set as a fire boulder in the editor. Need to create fire to place on floor
      (if (Variables|Default|GetFireBoulder)
        (bind _returnvalue (Utilities|Time|SetTimerbyEvent (delegate Custom|LeaveFireTrail) 0.2 true))
        (Variables|Default|SetFireTrailTimer _returnvalue)
        (CallFunction|Roll)
        (else
          (CallFunction|Roll))))))

(event Custom|GainSpeed
  ;[1 1 1] Gradually increase speed of boulder the longer it is rolling without hitting anything
  (if (<= (Variables|Default|GetBoulderCurrentSpeed) (Variables|Default|GetBoulderMaxSpeed))
    (bind _output_get (Variables|Default|SetBoulderCurrentSpeed (+ (Variables|Default|GetBoulderCurrentSpeed) 0.05)))
    (Components|Timeline|SetPlayRate (Variables|Default|GetTL_Roll) _output_get)))

(event Custom|Roll
  ;[1 1 1] Start rolling. Starts off slow
  (bind _returnvalue (Utilities|Time|SetTimerbyEvent (delegate Custom|GainSpeed) 0.1 true))
  (bind _alpha (Timeline|TL_Roll Play)
    (:Update
      (Transformation|SetActorLocation (Math|Vector|Lerp(Vector) (Variables|Default|GetStartPosition) (Variables|Default|GetTargetPosition) _alpha) false false))
    (:Finished
      (Utilities|Time|ClearandInvalidateTimerbyHandle _returnvalue)
      (if (Variables|Default|GetFireBoulder)
        (Utilities|Time|ClearandInvalidateTimerbyHandle (Variables|Default|GetFireTrailTimer))))))

(event Custom|LeaveFireTrail
  (bind _returnvalue (Transformation|GetActorLocation))
  ;[1 1 1] Started working on leaving a trail of fire if it is set as a fire boulder in the editor. Need to create fire to place on floor
  (Utilities|Array|Add (Variables|Default|GetFireTrailPoints) _returnvalue)
  (Rendering|Debug|DrawDebugCircle _returnvalue 1e+02 100 "(R=1.000000,G=1.000000,B=1.000000,A=1.000000)" 1e+02 1.0 "1.000000,0.000000,0.000000" "0.000000,1.000000,0.000000"))

(event EventBeginPlay
  ;[1 1 1] Set starting position of boulder (needed for lerp)
  (Variables|Default|SetStartPosition (Transformation|GetActorLocation))
  (Components|Timeline|SetPlayRate (Variables|Default|GetTL_Roll) 0.2))

(fn ConstructionScript)